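; Enemy character AI that patrols, chases the player on sight and attacks in melee.
; Patrol loops AIMoveTo toward random reachable points around the player's location at walking speed.
; PawnSensing sightings trigger a faster chase that refills a retry counter, returning to patrol when it runs out.
; Reaching the player plays a hit montage; a separate Ataque event plays a grunt and damages via right-hand sphere trace.
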(event OnSeePawn(PawnSensing)
  (params (Pawn :type Pawn%20Object%20Reference))
  (bind _mesh (Variables|Character|GetMesh))
  (bind _returnvalue (Components|SkeletalMesh|GetAnimInstance _mesh))
  (bind _returnvalue_2 (Class|AnimInstance|IsAnyMontagePlaying _returnvalue))
  ;[1 1 1] Funcion para seguir al personaje
  (bind _asbp_character (Utilities|Casting|CastToBP_CHaracter Pawn))
  (Variables|Default|SetIntentosPerseguir 5)
  (Variables|Default|SetJugadorPerseguir _asbp_character)
  (CallFunction|CambiarVelocidad 2.7e+02 :!label _label)
  (if _returnvalue_2
    (if (> (Variables|Default|GetIntentosPerseguir) 0) :!label _label_2
      (Utilities|FlowControl|RetriggerableDelay 2.0)
      (Variables|Default|SetIntentosPerseguir (- (Variables|Default|GetIntentosPerseguir) 1))
      (goto _label)
      (else
        (CallFunction|Patrullar)))
    (else
      (AI|AIMoveTo self (Transformation|GetActorLocation (Variables|Default|GetJugadorPerseguir)) (Variables|Default|GetJugadorPerseguir) 1e+02 false
        (:then
          (goto _label_2))
        (:OnSuccess
          (if (not _returnvalue_2)
            (Animation|Montage|PlayMontage (Variables|Character|GetMesh) "/Game/Characters/Monster/Animations/Hit_montage.Hit_montage")))))))

(event Custom|Cambiar%20Velocidad
  (params (Velocidad :type Float%20%28single-precision%29))
  ;[1 1 1] Funcion para seguir al personaje
  (Variables|/Script/Engine.CharacterMovementComponent|SetMaxWalkSpeed (Variables|Character|GetCharacterMovement) Velocidad))

(event Custom|Patrullar
  ;[1 1 1] Funcion para Patrullar
  (if (not (> (Variables|Default|GetIntentosPerseguir) 0)) :!label _label
    (CallFunction|CambiarVelocidad 135.0)
    (AI|AIMoveTo self (.RandomLocation (AI|Navigation|GetRandomReachablePointinRadius (Transformation|GetActorLocation (Game|Player|GetPlayerPawn 0)) 1e+04 0 0)) 0 1e+02 false
      (:OnSuccess
        _)
      (:OnFail
        _))
    (Utilities|FlowControl|Delay 2.0)
    (goto _label)))

(event Custom|Ataque
  (bind _mesh (Variables|Character|GetMesh))
  (bind _returnvalue (Transformation|GetSocketLocation _mesh "RightHandIndex4"))
  (Audio|PlaySoundatLocation "/Game/Sounds/ScarySounds/michael-klier__large-monster-grunt-hit-02.michael-klier__large-monster-grunt-hit-02" (Transformation|GetActorLocation) "0, 0, 0" 1.0 1.0 0.0 0 0 0)
  (bind (_outhit _returnvalue_2) (Collision|SphereTraceByChannel _returnvalue _returnvalue 1e+02 "TraceTypeQuery2" false 0 "None" true "(R=1.000000,G=0.000000,B=0.000000,A=1.000000)" "(R=0.000000,G=1.000000,B=0.000000,A=1.000000)" 0.0))
  (if _returnvalue_2
    (Game|Damage|ApplyDamage (.HitActor (Collision|BreakHitResult _outhit)) 51.0 (Game|GetInstigatorController (.HitActor (Collision|BreakHitResult _outhit))) self)))

(event Collision|EventActorBeginOverlap
  (params (OtherActor :type Actor%20Object%20Reference)))

(event EventTick
  (params (DeltaSeconds :type Float%20%28single-precision%29)))

(event EventBeginPlay
  ;[1 1 1] Funcion para Patrullar
  (CallFunction|Patrullar))

(fn ConstructionScript)