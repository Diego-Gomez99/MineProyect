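; Generator actor that the player switches on by holding the interact input inside its trigger box.
; Box overlap shows the prompt and toggles input; holding fills a progress bar through a Delay-throttled axis event, and releasing resets it.
; Completion notifies MyGamemode's counter, disables the box, briefly shows a count widget and starts the lighting sequence.
; That sequence plays a sound and uses chained delays to flicker lights and swap halogen materials.
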(event OnComponentBeginOverlap(Box)
  (params (OverlappedComponent :type Primitive%20Component%20Object%20Reference) (OtherActor :type Actor%20Object%20Reference) (OtherComp :type Primitive%20Component%20Object%20Reference) (OtherBodyIndex :type Integer) (bFromSweep :type Boolean) (SweepResult :type Hit%20Result%20Structure%20%28by%20ref%29))
  ;[1 0.7487 0.07902] Mecanica Encender Generador
  (bind _asbp_character (Utilities|Casting|CastToBP_CHaracter OtherActor))
  (Variables|/Game/Blueprints/MyCharacter/BP_CHaracter.BP_CHaracter_C|SetText _asbp_character "Press \"E\" to interact")
  (Input|EnableInput (Game|GetPlayerController 0)))

(event OnComponentEndOverlap(Box)
  (params (OverlappedComponent :type Primitive%20Component%20Object%20Reference) (OtherActor :type Actor%20Object%20Reference) (OtherComp :type Primitive%20Component%20Object%20Reference) (OtherBodyIndex :type Integer))
  ;[1 0.7487 0.07902] Mecanica Encender Generador
  (bind _asbp_character (Utilities|Casting|CastToBP_CHaracter OtherActor))
  (Variables|/Game/Blueprints/MyCharacter/BP_CHaracter.BP_CHaracter_C|SetText _asbp_character "")
  (Input|DisableInput (Game|GetPlayerController 0)))

(event Custom|ShowGeneratorBar
  ;[0.2129 1 0.3265] Mostrar barra de progreso del generador
  (Widget|SetVisibility (Variables|Default|GetGeneratorProcessBarReference) "Visible"))

(event Custom|HideGeneratorBar
  ;[0.2129 1 0.3265] Mostrar barra de progreso del generador
  (Widget|SetVisibility (Variables|Default|GetGeneratorProcessBarReference) "Hidden"))

(event Custom|GeneratorTurnedOn
  (bind _generatorcountreference (Variables|Default|GetGeneratorCountReference))
  ;[1 0.2102 0.1565] Cuando el Generador esté encendido
  (Collision|SetCollisionObjectType (Variables|Debug|GetStaticMeshComponent) "ECC_Pawn")
  (Widget|RemovefromParent (Variables|Default|GetGeneratorProcessBarReference))
  (bind _asmy_gamemode (Utilities|Casting|CastToMyGamemode (Game|GetGameMode)))
  (Default|GeneratorCounterEvent _asmy_gamemode)
  (Collision|SetCollisionEnabled (Variables|Default|GetBox) "NoCollision")
  (Widget|SetVisibility _generatorcountreference "Visible")
  (CallFunction|EncenderLuces)
  (Utilities|FlowControl|Delay 3.0)
  (Widget|SetVisibility _generatorcountreference "Hidden"))

(event Custom|Encender_Luces
  (Audio|Components|Audio|Play (Variables|Default|GetGenerator_On) 0.0)
  (Utilities|FlowControl|Delay 0.5)
  (Rendering|SetVisibility (Variables|Default|GetRectLight) true false)
  (Rendering|Material|SetMaterial (Variables|Default|Getgenerator_skfb_zlaczka_lp) 0 "/Game/MyMeshes/Generator/halogen_on.halogen_on")
  (Utilities|FlowControl|Delay 0.5)
  (Rendering|Components|Light|SetIntensity (Variables|Default|GetRectLight1) 0.0)
  (Rendering|Material|SetMaterial (Variables|Default|Getgenerator_skfb_zlaczka_lp) 0 "/Game/MyMeshes/Generator/halogen_off.halogen_off")
  (Utilities|FlowControl|Delay 0.3)
  (Rendering|Components|Light|SetIntensity (Variables|Default|GetRectLight1) 1e+03)
  (Rendering|Material|SetMaterial (Variables|Default|Getgenerator_skfb_zlaczka_lp) 0 "/Game/MyMeshes/Generator/halogen_on.halogen_on")
  (Utilities|FlowControl|Delay 0.2)
  (Rendering|Components|Light|SetIntensity (Variables|Default|GetRectLight1) 1e+01)
  (Rendering|Material|SetMaterial (Variables|Default|Getgenerator_skfb_zlaczka_lp) 0 "/Game/MyMeshes/Generator/halogen_off.halogen_off")
  (Utilities|FlowControl|Delay 0.1)
  (Rendering|Components|Light|SetIntensity (Variables|Default|GetRectLight1) 5e+03)
  (Rendering|Material|SetMaterial (Variables|Default|Getgenerator_skfb_zlaczka_lp) 0 "/Game/MyMeshes/Generator/halogen_on.halogen_on"))

(event EventBeginPlay
  ;[0.4025 0.1661 1] Setear los elementos UI del generador
  (bind _returnvalue (UserInterface|CreateWidget "/Game/UI/GeneratorBar_UI.GeneratorBar_UI_C"))
  (bind _output_get (Variables|Default|SetGeneratorProcessBarReference _returnvalue))
  (UserInterface|Viewport|AddtoViewport _output_get 0)
  (Widget|SetVisibility (Variables|Default|GetGeneratorProcessBarReference) "Hidden")
  (bind _returnvalue_2 (UserInterface|CreateWidget "/Game/UI/GeneratorCount_UI.GeneratorCount_UI_C"))
  (bind _output_get_2 (Variables|Default|SetGeneratorCountReference _returnvalue_2))
  (UserInterface|Viewport|AddtoViewport _output_get_2 0)
  (Widget|SetVisibility (Variables|Default|GetGeneratorCountReference) "Hidden"))

(event Input|AxisEvents|InputAxisGenerator
  (params (AxisValue :type Float%20%28single-precision%29))
  ;[1 0.7487 0.07902] Mecanica Encender Generador
  (if (== AxisValue 1.0)
    (CallFunction|ShowGeneratorBar)
    (Utilities|FlowControl|Delay 0.1)
    (Variables|Default|SetGeneratorProgress (+ (Variables|Default|GetGeneratorProgress) 0.1))
    (if (>= (Variables|Default|GetGeneratorProgress) 1.0)
      (Variables|Default|SetGeneratorProgress 0.0)
      (CallFunction|GeneratorTurnedon))
    (else
      (CallFunction|HideGeneratorBar)
      (Variables|Default|SetGeneratorProgress 0.0))))

(fn ConstructionScript)