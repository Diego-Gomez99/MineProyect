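; Elevator actor that starts moving automatically on BeginPlay, with a positioned movement sound.
; The MovimientoElevador timeline sets its location each update by subtracting the track value from the starting position.
; A delay chain on that same Update pin later flickers the spot and point lights through changing intensities, then hides them.
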(event EventBeginPlay
  (Utilities|FlowControl|Sequence
    (:then_0
      (Audio|PlaySoundatLocation "/Game/Sounds/ElevatorCUE.ElevatorCUE" "0, 0, 0" "0, 0, 0" 1.0 1.0 0.0 "/Game/Sounds/ElevatorMoveAttenuation.ElevatorMoveAttenuation" 0 0))
    (:then_1
      (bind _output_get (Variables|Default|SetPosicionElevador (Transformation|GetActorLocation)))
      (bind _movimineto (Timeline|MovimientoElevador Play)
        (:Update
          (Transformation|SetActorLocation (- _output_get _movimineto) false false)
          (Utilities|FlowControl|Delay 25.0)
          (Rendering|Components|Light|SetIntensity (Variables|Default|GetSpotLight) 1.5e+03)
          (Utilities|FlowControl|Delay 0.2)
          (Rendering|Components|Light|SetIntensity (Variables|Default|GetSpotLight) 4e+03)
          (Utilities|FlowControl|Delay 0.2)
          (Rendering|Components|Light|SetIntensity (Variables|Default|GetSpotLight) 5e+02)
          (Utilities|FlowControl|Delay 0.2)
          (Rendering|Components|Light|SetIntensity (Variables|Default|GetSpotLight) 5e+03)
          (Utilities|FlowControl|Delay 0.2)
          (Rendering|Components|Light|SetIntensity (Variables|Default|GetSpotLight) 1.5e+03)
          (Utilities|FlowControl|Delay 0.2)
          (Rendering|SetVisibility (Variables|Default|GetPointLight) false false))))))

(event Collision|EventActorBeginOverlap
  (params (OtherActor :type Actor%20Object%20Reference)))

(event EventTick
  (params (DeltaSeconds :type Float%20%28single-precision%29)))

(fn ConstructionScript)