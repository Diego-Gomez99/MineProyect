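; BP_LOOCKERTEST is an interactable pickup that grants the player the ability to turn on a light, apparently a flashlight.
; A Box overlap with BP_CHaracter shows an interact prompt through the character's Text and enables input on the actor; leaving clears both.
; Pressing the Action input sets CanTurnlight on MyPlayerController and destroys the actor.
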(event OnComponentBeginOverlap(Box)
  (params (OverlappedComponent :type Primitive%20Component%20Object%20Reference) (OtherActor :type Actor%20Object%20Reference) (OtherComp :type Primitive%20Component%20Object%20Reference) (OtherBodyIndex :type Integer) (bFromSweep :type Boolean) (SweepResult :type Hit%20Result%20Structure%20%28by%20ref%29))
  ;[1 1 1] Mecanica tomar linterna
  (bind _asbp_character (Utilities|Casting|CastToBP_CHaracter OtherActor))
  (Variables|/Game/Blueprints/MyCharacter/BP_CHaracter.BP_CHaracter_C|SetText _asbp_character "Press \"E\" to interact")
  (Input|EnableInput (Game|GetPlayerController 0)))

(event OnComponentEndOverlap(Box)
  (params (OverlappedComponent :type Primitive%20Component%20Object%20Reference) (OtherActor :type Actor%20Object%20Reference) (OtherComp :type Primitive%20Component%20Object%20Reference) (OtherBodyIndex :type Integer))
  ;[1 1 1] Mecanica tomar linterna
  (bind _asbp_character (Utilities|Casting|CastToBP_CHaracter OtherActor))
  (Variables|/Game/Blueprints/MyCharacter/BP_CHaracter.BP_CHaracter_C|SetText _asbp_character "")
  (Input|DisableInput (Game|GetPlayerController 0)))

(event Input|ActionEvents|InputActionAction
  (params (Key :type Key%20Structure :default "None"))
  ;[1 1 1] Mecanica tomar linterna
  (:Pressed
    (bind _asmy_player_controller (Utilities|Casting|CastToMyPlayerController (Game|GetPlayerController 0)))
    (Variables|/Game/Blueprints/MyCharacter/MyPlayerController.MyPlayerController_C|SetCanTurnlight _asmy_player_controller true)
    (Actor|DestroyActor)))

(fn ConstructionScript)