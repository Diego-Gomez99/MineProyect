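; Elevator actor that starts moving on BeginPlay with positioned sound and stages a lighting failure during the ride.
; The MovimientoElevador timeline subtracts its track value from the stored start location to move the actor.
; Each timeline update calls LightsTurnOff, whose delay chain flickers the spot and point lights, then hides them and swaps the fixture materials to unlit.
; LightsTurnOn restores intensity and visibility but is not called here.
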(event Custom|LightsTurnOff
  ;[1 1 1] Secuencia para apagar las luces
  (Utilities|FlowControl|Delay 25.0)
  (Rendering|Components|Light|SetIntensity (Variables|Default|GetSpotLight) 1.5e+03)
  (Utilities|FlowControl|Delay 0.2)
  (Rendering|Components|Light|SetIntensity (Variables|Default|GetSpotLight) 4e+03)
  (Utilities|FlowControl|Delay 0.2)
  (Rendering|Components|Light|SetIntensity (Variables|Default|GetSpotLight) 5e+02)
  (Utilities|FlowControl|Delay 0.2)
  (Rendering|Components|Light|SetIntensity (Variables|Default|GetSpotLight) 5e+03)
  (Utilities|FlowControl|Delay 0.2)
  (Rendering|Components|Light|SetIntensity (Variables|Default|GetSpotLight) 1.5e+03)
  (Utilities|FlowControl|Delay 0.2)
  (Rendering|SetVisibility (Variables|Default|GetPointLight) false false)
  (Rendering|Material|SetMaterial (Variables|Default|GetLight_Mesh) 0 "/Game/MyMaterials/MT_LightningOff.MT_LightningOff"))

(event Custom|LightsTurnOn
  (Rendering|Components|Light|SetIntensity (Variables|Default|GetSpotLight) 5e+03)
  (Rendering|SetVisibility (Variables|Default|GetPointLight) true false))

(event EventBeginPlay
  ;[1 1 1] Movimiento del elevador
  (Utilities|FlowControl|Sequence
    (:then_0
      (Audio|PlaySoundatLocation "/Game/Sounds/ElevatorCUE.ElevatorCUE" "0, 0, 0" "0, 0, 0" 1.0 1.0 0.0 "/Game/Sounds/ElevatorMoveAttenuation.ElevatorMoveAttenuation" 0 0))
    (:then_1
      (bind _output_get (Variables|Default|SetPosicionElevador (Transformation|GetActorLocation)))
      (bind _movimineto (Timeline|MovimientoElevador Play)
        (:Update
          (Transformation|SetActorLocation (- _output_get _movimineto) false false)
          (CallFunction|LightsTurnOff))))))

(fn ConstructionScript)