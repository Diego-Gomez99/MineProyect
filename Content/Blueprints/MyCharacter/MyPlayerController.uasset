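; Player controller that drives BP_CHaracter's movement, camera look and flashlight toggle.
; On BeginPlay it casts and caches the player character, then forwards look axes as pitch and yaw input.
; Movement axes add input along the forward and right vectors of the control rotation.
; The Flashlight action uses a FlipFlop to show or hide the character's light, playing switch on and off sounds.
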(event EventBeginPlay
  ;[1 1 1] Agregar Variable del Character
  (bind _asbp_character (Utilities|Casting|CastToBP_CHaracter (Game|GetPlayerCharacter 0)))
  (Variables|Default|SetMyCharacter _asbp_character))

(event Input|ActionEvents|InputActionFlashlight
  (params (Key :type Key%20Structure :default "None"))
  (bind _mycharacter (Variables|Default|GetMyCharacter))
  (bind _flashlight (Variables|/Game/Blueprints/MyCharacter/BP_CHaracter.BP_CHaracter_C|GetFlashlight _mycharacter))
  ;[1 0 0.1609] Mecanica Linterna
  (:Pressed
    (Utilities|FlowControl|FlipFlop
      (:A
        (Rendering|SetVisibility _flashlight true false)
        (Audio|PlaySound2D "/Game/Sounds/LampSwitchOn.LampSwitchOn" 1.0 1.0 0.0 0 0))
      (:B
        (Rendering|SetVisibility _flashlight false false)
        (Audio|PlaySound2D "/Game/Sounds/LampSwitchOff.LampSwitchOff" 1.0 1.0 0.0 0 0)))))

(event Input|AxisEvents|InputAxisLookUpDown
  (params (AxisValue :type Float%20%28single-precision%29))
  ;[1 1 1] Movimiento de la Cámara
  (Pawn|Input|AddControllerPitchInput (Variables|Default|GetMyCharacter) AxisValue))

(event Input|AxisEvents|InputAxisLookRightLeft
  (params (AxisValue :type Float%20%28single-precision%29))
  ;[1 1 1] Movimiento de la Cámara
  (Pawn|Input|AddControllerYawInput (Variables|Default|GetMyCharacter) AxisValue))

(event Input|AxisEvents|InputAxisMoveFowardBackward
  (params (AxisValue :type Float%20%28single-precision%29))
  (bind _mycharacter (Variables|Default|GetMyCharacter))
  ;[0.9545 1 0] Movimiento del Jugador
  (Pawn|Input|AddMovementInput _mycharacter (Math|Vector|GetForwardVector (Pawn|GetControlRotation _mycharacter :!class /Script/Engine.Pawn)) AxisValue false))

(event Input|AxisEvents|InputAxisMoveRightLeft
  (params (AxisValue :type Float%20%28single-precision%29))
  (bind _mycharacter (Variables|Default|GetMyCharacter))
  ;[0.9545 1 0] Movimiento del Jugador
  (Pawn|Input|AddMovementInput _mycharacter (Math|Vector|GetRightVector (Pawn|GetControlRotation _mycharacter :!class /Script/Engine.Pawn)) AxisValue false))

(fn ConstructionScript)