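; Player character Blueprint that highlights interactable objects in view and tracks health.
; Each Tick a camera sphere trace stores the hit and enables Custom Depth on the actor's "Outline"-tagged component.
; A DoOnce clears it when the trace misses; switching targets leaves the old actor highlighted, as StartTracing sets both true.
; AnyDamage lowers and prints clamped Salud (health); the delayed jumpscare sound and UI widget logic is unwired.
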(event OnComponentActivated(Flashlight)
  (params (Component :type Actor%20Component%20Object%20Reference) (bReset :type Boolean)))

(event EventBeginPlay)

(event EventTick
  (params (DeltaSeconds :type Float%20%28single-precision%29))
  (bind _camera (Variables|Default|GetCamera))
  (bind _returnvalue (Transformation|GetWorldLocation _camera))
  (bind (_outhit _returnvalue_2) (Collision|SphereTraceForObjects _returnvalue (+ _returnvalue (* (Math|Vector|GetForwardVector _camera) (Variables|Default|GetRange))) (Variables|Default|GetRadius) (Utilities|Array|MakeArray "ObjectTypeQuery7") false 0 "None"))
  (if _returnvalue_2
    (if (== (.hitactor (Variables|Default|GetInteractable)) (.HitActor (Collision|BreakHitResult _outhit)))
      _
      (else
        (CallFunction|StartTracing (.HitActor (Collision|BreakHitResult _outhit)) (.hitactor (Variables|Default|GetInteractable)))))
    (Variables|Default|SetInteractable _outhit)
    (goto _label Reset)
    (else
      (Utilities|FlowControl|DoOnce false :!label _label
        (:Completed
          (CallFunction|StopTracing))))))

(event Game|Damage|EventAnyDamage
  (params (Damage :type Float%20%28single-precision%29) (DamageType :type Damage%20Type%20Object%20Reference) (InstigatedBy :type Controller%20Object%20Reference) (DamageCauser :type Actor%20Object%20Reference))
  (bind _output_get (Variables|Default|SetSalud (Math|Float|Clamp(Float) (- (Variables|Default|GetSalud) Damage) 0.0 1e+02)))
  (Development|PrintString (Utilities|String|ToString(Float) _output_get)))

(fn ConstructionScript)

(fn StartTracing
  (params (newActor :type Actor%20Object%20Reference) (oldActor :type Actor%20Object%20Reference))
  (Rendering|SetRenderCustomDepth (Utilities|Array|Get(acopy) (Actor|GetComponentsbyTag newActor "/Script/Engine.PrimitiveComponent" "Outline")) true)
  (if (not (== oldActor 0))
    (Rendering|SetRenderCustomDepth (Utilities|Array|Get(acopy) (Actor|GetComponentsbyTag oldActor "/Script/Engine.PrimitiveComponent" "Outline")) true)))

(fn StopTracing
  (Utilities|FlowControl|Sequence
    (:then_0
      (if (not (== (.hitactor (Variables|Default|GetInteractable)) 0))
        (Rendering|SetRenderCustomDepth (Utilities|Array|Get(acopy) (Actor|GetComponentsbyTag (.hitactor (Variables|Default|GetInteractable)) "/Script/Engine.PrimitiveComponent" "Outline")) false)))
    (:then_1
      (Variables|Default|SetInteractable ""))))