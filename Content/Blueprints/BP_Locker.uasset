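; BP_Locker is a locker Frank can hide in, toggled by the Action input while he overlaps its Box.
; Overlap shows a prompt and opens a Gate; each press runs ToggleHide and a door timeline.
; ToggleHide switches Frank's visibility, movement and collision, blends the view between Frank and locker, and toggles the locker lights.
; A separate IA_AbrePuerta event swings the door through its own timeline with an opening sound.
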(event OnComponentBeginOverlap(Box)
  (params (OverlappedComponent :type Primitive%20Component%20Object%20Reference) (OtherActor :type Actor%20Object%20Reference) (OtherComp :type Primitive%20Component%20Object%20Reference) (OtherBodyIndex :type Integer) (bFromSweep :type Boolean) (SweepResult :type Hit%20Result%20Structure%20%28by%20ref%29))
  (bind _asbp_frank (Utilities|Casting|CastToBP_Frank OtherActor))
  (bind _output_get (Variables|Default|SetFrank _asbp_frank))
  (Variables|/Game/Blueprints/MyCharacter/BP_Frank.BP_Frank_C|SetText _output_get "E to hide")
  (Input|EnableInput (Game|GetPlayerController 0))
  (Utilities|FlowControl|Gate true) ; enters at Open
)

(event OnComponentEndOverlap(Box)
  (params (OverlappedComponent :type Primitive%20Component%20Object%20Reference) (OtherActor :type Actor%20Object%20Reference) (OtherComp :type Primitive%20Component%20Object%20Reference) (OtherBodyIndex :type Integer))
  (bind _returnvalue (Game|GetPlayerController 0))
  (bind _asbp_frank (Utilities|Casting|CastToBP_Frank OtherActor))
  (Variables|/Game/Blueprints/MyCharacter/BP_Frank.BP_Frank_C|SetText _asbp_frank "")
  (Input|DisableInput _returnvalue)
  (Utilities|FlowControl|Gate true) ; enters at Close
)

(event Custom|IA_AbrePuerta
  (bind _doortrack (Timeline|Timeline_0 PlayFromStart)
    (:Update
      (Transformation|SetRelativeRotation (Variables|Default|GetLockerDoor) (Math|Rotator|MakeRotator 0.0 0.0 (Math|Float|Lerp (Variables|Default|GetAnguloPuertaCerrada) (Variables|Default|GetAnguloPuertaAbierta) _doortrack)) false false)
      (Utilities|FlowControl|DoOnce false
        (:Completed
          (Audio|PlaySoundatLocation "/Game/Sounds/LockerOpen.LockerOpen" (Transformation|GetActorLocation) "0, 0, 0" 1.0 1.0 0.0 0 0 0))))))

(event Input|ActionEvents|InputActionAction
  (params (Key :type Key%20Structure :default "None"))
  (:Pressed
    (Audio|Components|Audio|Play (Variables|Default|GetOpenCloseLocker) 0.0)
    (Utilities|FlowControl|Gate true :!label _label
      (:Exit
        (Utilities|FlowControl|Sequence
          (:then_0
            (CallFunction|ToggleHide)
            (Utilities|FlowControl|Delay 0.2)
            (Input|EnableInput (Game|GetPlayerController 0))
            (goto _label Open))
          (:then_1
            (|AnimOpenCloseDoor)))))))

(fn ConstructionScript)

(fn ToggleHide
  (bind _returnvalue (Game|GetPlayerController 0))
  (bind _spotlight (Variables|Default|GetSpotLight))
  (bind _frank (Variables|Default|GetFrank))
  (bind _charactermovement (Variables|/Script/Engine.Character|GetCharacterMovement _frank))
  (if (Variables|Default|GetIshiding?)
    (Variables|Default|SetIshiding? false)
    (Rendering|SetActorHiddenInGame _frank false)
    (Pawn|Components|CharacterMovement|SetMovementMode _charactermovement "MOVE_Walking" 0)
    (Collision|SetActorEnableCollision _frank true)
    (Game|Player|SetViewTargetwithBlend _returnvalue _frank 0.3 "VTBlend_Linear" 0.0 false)
    (Rendering|SetVisibility _spotlight false false)
    (else
      (Variables|Default|SetIshiding? true)
      (Rendering|SetActorHiddenInGame _frank true)
      (Pawn|Components|CharacterMovement|DisableMovement _charactermovement)
      (Collision|SetActorEnableCollision _frank false)
      (Game|Player|SetViewTargetwithBlend _returnvalue self 0.3 "VTBlend_Linear" 0.0 false)
      (Rendering|SetVisibility _spotlight true false))))